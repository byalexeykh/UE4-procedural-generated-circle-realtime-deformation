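; Player controller Blueprint that turns press-and-drag touch input into world coordinates for the game.
; Press and release actions toggle IsPressed; a press traces immediately, and the TouchInputAxis event repeats the trace while held.
; Each trace deprojects the mouse position along a short Visibility ray and hands the impact point's Y and Z to PassCoordsToCode, ignoring X and whether anything was hit.
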(event Input|ActionEvents|InputActionTouchInputMappings
  (params (Key :type Key%20Structure))
  (bind (_worldlocation _worlddirection) (Game|Player|ConvertMouseLocationToWorldSpace))
  (:Pressed
    (Variables|Default|SetisPressed true)
    (bind _outhit (Collision|LineTraceByChannel _worldlocation (+ _worldlocation (* _worlddirection 1000)) "TraceTypeQuery1" false 0 "None"))
    (Class|MyPlayerController|PassCoordstoCode (.Y (Math|Vector|BreakVector (.ImpactPoint (Collision|BreakHitResult _outhit)))) (.Z (Math|Vector|BreakVector (.ImpactPoint (Collision|BreakHitResult _outhit))))))
  (:Released
    (Variables|Default|SetisPressed false)))

(event Input|AxisEvents|InputAxisTouchInputAxis
  (params (AxisValue :type Float%20%28single-precision%29))
  (bind (_worldlocation _worlddirection) (Game|Player|ConvertMouseLocationToWorldSpace))
  (if (Variables|Default|GetisPressed)
    (bind _outhit (Collision|LineTraceByChannel _worldlocation (+ _worldlocation (* _worlddirection 1000)) "TraceTypeQuery1" false 0 "None"))
    (Class|MyPlayerController|PassCoordstoCode (.Y (Math|Vector|BreakVector (.ImpactPoint (Collision|BreakHitResult _outhit)))) (.Z (Math|Vector|BreakVector (.ImpactPoint (Collision|BreakHitResult _outhit)))))))

(fn ConstructionScript)